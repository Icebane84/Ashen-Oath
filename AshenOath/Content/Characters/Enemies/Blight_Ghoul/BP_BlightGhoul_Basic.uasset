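; Basic Blight Ghoul enemy that moves toward the player and deals damage on contact.
; On BeginPlay it binds to its health component's death event and issues a single AIMoveTo targeting the first player character.
; Its box collision applies fixed damage through the health component of any overlapping AshenCombatCharacter.
; When its own health component reports death, the actor is destroyed immediately.
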(event OnComponentBeginOverlap(BoxCollision)
  (params (OverlappedComponent :type Primitive%20Component%20Object%20Reference) (OtherActor :type Actor%20Object%20Reference) (OtherComp :type Primitive%20Component%20Object%20Reference) (OtherBodyIndex :type Integer) (bFromSweep :type Boolean) (SweepResult :type Hit%20Result%20Structure%20%28by%20ref%29))
  (bind _asashen_combat_character (Utilities|Casting|CastToAshenCombatCharacter OtherActor))
  (Class|AshenOathHealthComponent|ReceiveDamage (Actor|GetComponentbyClass _asashen_combat_character "/Script/AshenOath.AshenOath_HealthComponent") 8e+01 0))

(event Custom|OnEnemyDied
  (Actor|DestroyActor))

(event EventBeginPlay
  (EventDispatchers|BindEventtoOnDied (Actor|GetComponentbyClass "/Script/AshenOath.AshenOath_HealthComponent") (delegate Custom|OnEnemyDied))
  (AI|AIMoveTo self "0, 0, 0" (Game|GetPlayerCharacter 0) 5e+01 false))

(event Collision|EventActorBeginOverlap
  (params (OtherActor :type Actor%20Object%20Reference)))

(event EventTick
  (params (DeltaSeconds :type Float%20%28single-precision%29)))

(fn ConstructionScript
  (|CallParentFunction))